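; AC_RT_Drawer_WS is a component that stamps its owner's world position into a shared render target every tick.
; It gets the render target and world size from the AC_RT_Manager_WS component on a designated manager owner.
; Draw feeds normalized position, brush size and falloff into a dynamic instance of M_RT_Composite_WS, then draws that material to the render target.
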(event `self.ReceiveBeginPlay`
  (set `self.RenderTargetManager` (`Actor.GetComponentByClass` (`self.RenderTargetManagerOwner`) "/RenderTarget/WorldSpace/AC_RT_Manager_WS.AC_RT_Manager_WS_C")))

(event `self.ReceiveTick`
  (params (DeltaSeconds :type "Float (single-precision)"))
  (`self.Draw` (`Actor.K2_GetActorLocation` (`self.GetOwner`)) (`self.WorldSpaceSize`)))

(fn `Draw`
  (params (WorldSpacePosition :type "Vector Structure") (WorldSpaceSize :type "Float (single-precision)"))
  (locals (LocalMID :type "MaterialInstanceDynamic Object Reference"))
  (`/Engine/EditorBlueprintResources/StandardMacros.IsValid` (`self.RenderTargetManager`)
    (:`Is Valid`
      (`/Engine/EditorBlueprintResources/StandardMacros.Create and Assign MID` (`local.LocalMID`) "/RenderTarget/WorldSpace/M_RT_Composite_WS.M_RT_Composite_WS"
        (:`Out`
          (`MaterialInstanceDynamic.SetVectorParameterValue` (`local.LocalMID`) "World space position" (`KismetMathLibrary.Conv_VectorToLinearColor` (/ WorldSpacePosition (`/RenderTarget/WorldSpace/AC_RT_Manager_WS.WorldSize` (`self.RenderTargetManager`)))))
          (`MaterialInstanceDynamic.SetScalarParameterValue` (`local.LocalMID`) "World space size" (/ WorldSpaceSize (`KismetMathLibrary.Conv_IntToDouble` (`/RenderTarget/WorldSpace/AC_RT_Manager_WS.RenderTargetSize` (`self.RenderTargetManager`)))))
          (`MaterialInstanceDynamic.SetScalarParameterValue` (`local.LocalMID`) "FallOff" (`self.FallOff`))
          (`KismetRenderingLibrary.DrawMaterialToRenderTarget` (`/RenderTarget/WorldSpace/AC_RT_Manager_WS.RenderTarget` (`self.RenderTargetManager`)) (`local.LocalMID`)))))))